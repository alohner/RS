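; Weapon actor that damages destructible objects it hits.
; On Hit, it checks that the player pawn is CharacterAnto, casts the other actor to BP_DestructibleObjectAbstract and applies DammageOccur as damage, instigated by the first player controller.
; The branch before that cast is hard-wired true, and debug prints show the target's Life before damage.
; ActorBeginOverlap only prints a debug message.
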(event EventActorBeginOverlap
  (params (OtherActor :type Actor%20Object%20Reference))
  (Development|PrintString "Hello"))

(event EventHit
  (params (MyComp :type Primitive%20Component%20Object%20Reference) (Other :type Actor%20Object%20Reference) (OtherComp :type Primitive%20Component%20Object%20Reference) (bSelfMoved :type Boolean) (HitLocation :type Vector :default "0, 0, 0") (HitNormal :type Vector :default "0, 0, 0") (NormalImpulse :type Vector :default "0, 0, 0") (Hit :type Hit%20Result%20Structure%20%28by%20ref%29))
  (Utilities|Casting|CastToCharacterAnto (Game|GetPlayerCharacter 0))
  (if true
    (bind _asbp_destructibleobjectabstract_c (Utilities|Casting|CastToBP_DestructibleObjectAbstract Other))
    (Development|PrintString "Arbre")
    (Utilities|IsValid _asbp_destructibleobjectabstract_c
      (:Is%20Valid
        (Development|PrintString (Utilities|String|ToString(Integer) (Variables|/Game/BluePrintAntonin/BP_DestructibleObjectAbstract.BP_DestructibleObjectAbstract_C|GetLife _asbp_destructibleobjectabstract_c)))
        (Game|Damage|ApplyDamage _asbp_destructibleobjectabstract_c (Math|Conversions|ToFloat(Integer) (Variables|Default|GetDammageOccur)) (Game|GetPlayerController 0) self)))))

(fn ConstructionScript)